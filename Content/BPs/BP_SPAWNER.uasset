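; Spawner actor that periodically spawns one of four capture item Blueprints at a random point inside its Box component.
; BeginPlay plays a timeline that acts as a repeating timer.
; When it finishes, a random integer picks the item class, which spawns regardless of collision at a point from GetRandomPositionFromBox.
; RestartTimeline then replays the timeline from the start, looping indefinitely.
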(event Custom|RestartTimeline
  (Timeline|Timeline_0 PlayFromStart
    (:Finished
      (switch int (Math|Random|RandomInteger 4)
        (:0
          (Game|SpawnActorfromClass "/Game/BPs/BP_ITEM_CAPTURE_01.BP_ITEM_CAPTURE_01_C" (Math|Transform|MakeTransform (CallFunction|GetRandomPositionfromBox) "0, 0, 0" "1,1,1") "AlwaysSpawn" 0 0)
          (CallFunction|RestartTimeline))
        (:1
          (Game|SpawnActorfromClass "/Game/BPs/BP_ITEM_CAPTURE_02.BP_ITEM_CAPTURE_02_C" (Math|Transform|MakeTransform (CallFunction|GetRandomPositionfromBox) "0, 0, 0" "1,1,1") "AlwaysSpawn" 0 0)
          (CallFunction|RestartTimeline))
        (:2
          (Game|SpawnActorfromClass "/Game/BPs/BP_ITEM_CAPTURE_03.BP_ITEM_CAPTURE_03_C" (Math|Transform|MakeTransform (CallFunction|GetRandomPositionfromBox) "0, 0, 0" "1,1,1") "AlwaysSpawn" 0 0)
          (CallFunction|RestartTimeline))
        (:3
          (Game|SpawnActorfromClass "/Game/BPs/BP_ITEM_CAPTURE_04.BP_ITEM_CAPTURE_04_C" (Math|Transform|MakeTransform (CallFunction|GetRandomPositionfromBox) "0, 0, 0" "1,1,1") "AlwaysSpawn" 0 0)
          (CallFunction|RestartTimeline))))))

(event EventBeginPlay
  (Timeline|Timeline_0 Play
    (:Finished
      (switch int (Math|Random|RandomInteger 4)
        (:0
          (Game|SpawnActorfromClass "/Game/BPs/BP_ITEM_CAPTURE_01.BP_ITEM_CAPTURE_01_C" (Math|Transform|MakeTransform (CallFunction|GetRandomPositionfromBox) "0, 0, 0" "1,1,1") "AlwaysSpawn" 0 0)
          (CallFunction|RestartTimeline))
        (:1
          (Game|SpawnActorfromClass "/Game/BPs/BP_ITEM_CAPTURE_02.BP_ITEM_CAPTURE_02_C" (Math|Transform|MakeTransform (CallFunction|GetRandomPositionfromBox) "0, 0, 0" "1,1,1") "AlwaysSpawn" 0 0)
          (CallFunction|RestartTimeline))
        (:2
          (Game|SpawnActorfromClass "/Game/BPs/BP_ITEM_CAPTURE_03.BP_ITEM_CAPTURE_03_C" (Math|Transform|MakeTransform (CallFunction|GetRandomPositionfromBox) "0, 0, 0" "1,1,1") "AlwaysSpawn" 0 0)
          (CallFunction|RestartTimeline))
        (:3
          (Game|SpawnActorfromClass "/Game/BPs/BP_ITEM_CAPTURE_04.BP_ITEM_CAPTURE_04_C" (Math|Transform|MakeTransform (CallFunction|GetRandomPositionfromBox) "0, 0, 0" "1,1,1") "AlwaysSpawn" 0 0)
          (CallFunction|RestartTimeline))))))

(fn ConstructionScript)

(fn GetRandomPositionfromBox
  (bind _box (Variables|Default|GetBox))
  (bind (_origin _boxextent) (Collision|GetComponentBounds _box))
  (return (Math|Random|RandomPointinBoundingBox _origin _boxextent)))