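; Gameplay manager for a timed sequence-matching challenge, which also creates the main UBP_PRINCIPAL widget on BeginPlay.
; It fills Desafio with a random-length list of four possible enum items, and FnVerificaRemoveItem removes the front item when the submitted one matches.
; Clearing the list generates a new challenge, increments the completed count and resets the countdown.
; A looping one-second timer decrements the countdown and opens the game-over level at zero.
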(event EventBeginPlay
  (CallFunction|FnGeraDesafio)
  (bind _returnvalue (UserInterface|CreateWidget "/Game/HUD/UBP_PRINCIPAL.UBP_PRINCIPAL_C" (Game|GetPlayerController 0)))
  (UserInterface|Viewport|AddtoViewport _returnvalue 0)
  (Utilities|Time|SetTimerbyFunctionName 0 "fnDecrementaTimer" 1.0 true 1.0))

(fn ConstructionScript)

(fn FnGeraDesafio
  (Utilities|Array|Clear (Variables|Default|GetDesafio))
  (for _index (range 0 (Math|Random|RandomInteger 10))
    (switch int (Math|Random|RandomInteger 4)
      (:0
        (LocalVariables|SetItemDesafio "NewEnumerator0"))
      (:1
        (LocalVariables|SetItemDesafio "NewEnumerator1"))
      (:2
        (LocalVariables|SetItemDesafio "NewEnumerator2"))
      (:3
        (LocalVariables|SetItemDesafio "NewEnumerator3")))
    (Utilities|Array|Add (Variables|Default|GetDesafio) (LocalVariables|GetItemDesafio))))

(fn FnIncDesafioFinalizado
  (Variables|Default|SetDesafiosFinalizados (+ (Variables|Default|GetDesafiosFinalizados) 1)))

(fn FnVerificaRemoveItem
  (params (ItemToVerify :type E_ITEM_SELECAO%20Enum :default "NewEnumerator4"))
  (bind _desafio (Variables|Default|GetDesafio))
  (bind _output_get (LocalVariables|SetValuesAreEquals (Utilities|Enum|Equal(Enum) ItemToVerify (Utilities|Array|Get(acopy) (Variables|Default|GetDesafio)))))
  (if _output_get
    (Utilities|Array|RemoveIndex _desafio)
    (if (<= (Utilities|Array|Length _desafio) 0)
      (CallFunction|FnGeraDesafio)
      (CallFunction|FnIncDesafioFinalizado)
      (CallFunction|FnReiniciaTimer)))
  (return (LocalVariables|GetValuesAreEquals)))

(fn FnReiniciaTimer
  (Variables|Default|SetTimerValue 30))

(fn FnGameOver
  (if (<= (Variables|Default|GetTimerValue) 0)
    (Game|OpenLevel(byName) "/Game/Maps/L_GAME_OVER")))

(fn FnDecrementaTimer
  (Variables|Default|SetTimerValue (- (Variables|Default|GetTimerValue) 1))
  (CallFunction|FnGameOver))