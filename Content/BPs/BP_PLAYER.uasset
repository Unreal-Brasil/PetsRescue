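; BP_PLAYER is the player Blueprint for picking up and dragging objects with a visible mouse cursor.
; Left press stores the actor under the cursor and disables physics on BP_ITEM_CAPTURE_BASE items; release restores their physics and clears the selection.
; Tick moves any selected actor toward the cursor hit in X and Y and toward a fixed height, using DeltaSeconds as linear blend alpha for a lagging follow.
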(event EventBeginPlay
  (Variables|/Script/Engine.PlayerController|SetbShowMouseCursor (Game|GetPlayerController 0) true))

(event EventTick
  (params (DeltaSeconds :type Float%20%28single-precision%29))
  (bind _returnvalue (Game|GetPlayerController 0))
  (bind _selectedobject (Variables|Default|GetSelectedObject))
  (bind (_hitresult _returnvalue_2) (Game|Player|GetHitResultUnderCursorbyChannel _returnvalue "TraceTypeQuery1" true))
  (bind _returnvalue_3 (Transformation|GetActorLocation _selectedobject))
  (bind (_bblockinghit _binitialoverlap _time _distance _location _impactpoint _normal _impactnormal _physmat _hitactor) (Collision|BreakHitResult _hitresult))
  (bind (_x _y) (Math|Vector|BreakVector _location))
  (Utilities|IsValid _selectedobject
    (:Is%20Valid
      (if (Class|KismetMathLibrary|NotEqualExactlyVectorVector _location (Transformation|GetActorLocation _selectedobject))
        (Transformation|SetActorLocation (Variables|Default|GetSelectedObject) (Math|Vector|MakeVector (Math|Interpolation|Ease "Linear" DeltaSeconds (.x _returnvalue_3) _x) (Math|Interpolation|Ease "Linear" DeltaSeconds (.y _returnvalue_3) _y) (Math|Interpolation|Ease "Linear" DeltaSeconds (.z _returnvalue_3) 2.5e+02)) false false)))))

(event Input|MouseEvents|LeftMouseButton
  (params (Key :type Key%20Structure :default "None"))
  (bind _returnvalue (Game|GetPlayerController 0))
  (bind (_hitresult _returnvalue_2) (Game|Player|GetHitResultUnderCursorbyChannel _returnvalue "TraceTypeQuery1" true))
  (:Pressed
    (if _returnvalue_2
      (bind _output_get (Variables|Default|SetSelectedObject (.HitActor (Collision|BreakHitResult _hitresult))))
      (bind _asbp_item_capture_base (Utilities|Casting|CastToBP_ITEM_CAPTURE_BASE _output_get))
      (Physics|SetSimulatePhysics (Variables|/Game/BPs/BP_ITEM_CAPTURE_BASE.BP_ITEM_CAPTURE_BASE_C|GetObjectMesh _asbp_item_capture_base) false)))
  (:Released
    (bind _asbp_item_capture_base_2 (Utilities|Casting|CastToBP_ITEM_CAPTURE_BASE (Variables|Default|GetSelectedObject)))
    (Utilities|IsValid _asbp_item_capture_base_2
      (:Is%20Valid
        (Utilities|IsValid (Variables|/Game/BPs/BP_ITEM_CAPTURE_BASE.BP_ITEM_CAPTURE_BASE_C|GetObjectMesh _asbp_item_capture_base_2)
          (:Is%20Valid
            (Physics|SetSimulatePhysics (Variables|/Game/BPs/BP_ITEM_CAPTURE_BASE.BP_ITEM_CAPTURE_BASE_C|GetObjectMesh _asbp_item_capture_base_2) true)
            (Variables|Default|SetSelectedObject 0)))))))

(fn ConstructionScript)