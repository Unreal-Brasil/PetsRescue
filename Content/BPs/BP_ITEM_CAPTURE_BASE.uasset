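; BP_ITEM_CAPTURE_BASE is a base item actor that shows a countdown and destroys itself when time runs out.
; On BeginPlay it picks a random lifetime in seconds and starts a looping one-second timer bound by function name.
; Each tick of that timer updates the CountDown text, decrements the remaining time and prints it, or destroys the actor once it reaches zero.
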(event EventBeginPlay
  (Variables|Default|SetTimeUntilKill (Math|Random|RandomIntegerinRange 5 20))
  (CallFunction|FmExecuteTimer))

(event Collision|EventActorBeginOverlap
  (params (OtherActor :type Actor%20Object%20Reference)))

(event EventTick
  (params (DeltaSeconds :type Float%20%28single-precision%29)))

(fn ConstructionScript)

(fn FnTimertoKill
  (if (<= (Variables|Default|GetTimeUntilKill) 0)
    (Actor|DestroyActor)
    (else
      (Rendering|Components|TextRender|SetText (Variables|Default|GetCountDown) (Utilities|Text|ToText(Integer) (Variables|Default|GetTimeUntilKill)))
      (bind _output_get (Variables|Default|SetTimeUntilKill (- (Variables|Default|GetTimeUntilKill) 1)))
      (Development|PrintString (Utilities|String|ToString(Integer) _output_get)))))

(fn FmExecuteTimer
  (Utilities|Time|SetTimerbyFunctionName self "fnTimerToKill" 1.0 true))